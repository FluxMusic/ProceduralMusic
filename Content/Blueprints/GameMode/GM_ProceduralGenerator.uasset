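; Game mode that tests procedural drum and bass music by feeding generated patterns to an audio component.
; Construction creates BP_DrumAndBassGenerator; BlueprintTest runs it with a fixed seed, prints debug text and starts playback.
; Drum, bass, chord and melody data become float-array parameters, with PopulateChordArrays splitting chords by tone.
; BeginPlay is empty, and the sixth chord note overwrites the 9th arrays, leaving 11ths unfilled.
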(event `self.ReceiveBeginPlay`)

(fn `BlueprintTest`
  (bind _audio (`self.Audio`))
  (bind (_kickpattern _snarepattern _hhpattern _perc1pattern _perc2pattern _bassnotes _chordarrayout _melodypattern1) (`/Game/Blueprints/BP_DrumAndBassGenerator.GenerateMusic` (`self.DrumAndBassGenerator`) 7 (make `/Game/Blueprints/BPS_MusicGenSpecs` true false false "NewEnumerator0" "NewEnumerator1" "NewEnumerator0")))
  (for (_array_element _array_index) _kickpattern
    (`KismetSystemLibrary.PrintText` (`|FormatText` "{Index}: {Value}" _array_index _array_element) true true (struct :`R` 1.0 :`G` 0.444477 :`A` 1.0) 20.0))
  (`ActorComponent.Activate` _audio false)
  (`|ExecutionSequence`
    (:`then_0`
      (`AudioParameterControllerInterface.SetFloatArrayParameter` _audio "KickPattern" _kickpattern)
      (`KismetSystemLibrary.PrintString` "Set Kick Pattern"))
    (:`then_1`
      (`AudioParameterControllerInterface.SetFloatArrayParameter` _audio "SnarePattern" _snarepattern)
      (`KismetSystemLibrary.PrintString` "Set Snare Pattern"))
    (:`then_2`
      (`AudioParameterControllerInterface.SetFloatArrayParameter` _audio "HHPattern" _hhpattern)
      (`KismetSystemLibrary.PrintString` "Set HH Pattern"))
    (:`then_3`
      (`AudioParameterControllerInterface.SetFloatArrayParameter` _audio "Perc1Pattern" _perc1pattern)
      (`KismetSystemLibrary.PrintString` "Set Perc1 Pattern"))
    (:`then_4`
      (`AudioParameterControllerInterface.SetFloatArrayParameter` _audio "Perc2Pattern" _perc2pattern)
      (`KismetSystemLibrary.PrintString` "Set Perc2 Pattern"))
    (:`then_5`
      (for (_array_element_2 _array_index_2) _bassnotes
        (`KismetArrayLibrary.Array_Set` (`self.BassNotes`) _array_index_2 (break `/Game/Blueprints/BPS_MusicNote` _array_element_2) true)
        (`KismetArrayLibrary.Array_Set` (`self.BassVelocities`) _array_index_2 (`.Velocity_5_6DF5BD4448FA958C5E1D03A4550DEBD7` (break `/Game/Blueprints/BPS_MusicNote` _array_element_2)) true))
      (`AudioParameterControllerInterface.SetFloatArrayParameter` (`self.Audio`) "BassNotes" (`self.BassNotes`))
      (`AudioParameterControllerInterface.SetFloatArrayParameter` (`self.Audio`) "BassVelocities" (`self.BassVelocities`)))
    (:`then_6`
      (`self.PopulateChordArrays` _chordarrayout)
      (for (_array_element_3 _array_index_3) (`self.ChordRoots`)
        (`KismetSystemLibrary.PrintText` (`|FormatText` "Root: {RootNote}, Velocity: {RootVelocity} " _array_element_3 (`|GetArrayItem` (`self.ChordRootVelocities`) _array_index_3))))
      (for _array_element_4 (`self.Chord7ths`)
        (`KismetSystemLibrary.PrintText` (`|FormatText` "7th: {7th}, Velocity: {7thVelocity}" _array_element_4 (`|GetArrayItem` (`self.Chord7thVelocities`)))))
      (`AudioParameterControllerInterface.SetFloatArrayParameter` (`self.Audio`) "ChordRoots" (`self.ChordRoots`))
      (`AudioParameterControllerInterface.SetFloatArrayParameter` (`self.Audio`) "ChordRootVelocities" (`self.ChordRootVelocities`))
      (`AudioParameterControllerInterface.SetFloatArrayParameter` (`self.Audio`) "Chord3rds" (`self.Chord3rds`))
      (`AudioParameterControllerInterface.SetFloatArrayParameter` (`self.Audio`) "Chord3rdVelocities" (`self.Chord3rdVelocities`))
      (`AudioParameterControllerInterface.SetFloatArrayParameter` (`self.Audio`) "Chord5ths" (`self.Chord5ths`))
      (`AudioParameterControllerInterface.SetFloatArrayParameter` (`self.Audio`) "Chord5thVelocities" (`self.Chord5thVelocities`))
      (`AudioParameterControllerInterface.SetFloatArrayParameter` (`self.Audio`) "Chord7ths" (`self.Chord7ths`))
      (`AudioParameterControllerInterface.SetFloatArrayParameter` (`self.Audio`) "Chord7thVelocities" (`self.Chord7thVelocities`))
      (`AudioParameterControllerInterface.SetFloatArrayParameter` (`self.Audio`) "Chord9ths" (`self.Chord9ths`))
      (`AudioParameterControllerInterface.SetFloatArrayParameter` (`self.Audio`) "Chord9thVelocities" (`self.Chord9thVelocities`))
      (`AudioParameterControllerInterface.SetFloatArrayParameter` (`self.Audio`) "Chord11ths" (`self.Chord11ths`))
      (`AudioParameterControllerInterface.SetFloatArrayParameter` (`self.Audio`) "Chord11thVelocities" (`self.Chord11thVelocities`)))
    (:`then_7`
      (for (_array_element_5 _array_index_4) _melodypattern1
        (`KismetArrayLibrary.Array_Set` (`self.MelodyNotes`) _array_index_4 (break `/Game/Blueprints/BPS_MusicNote` _array_element_5) true)
        (`KismetArrayLibrary.Array_Set` (`self.MelodyVelocities`) _array_index_4 (`.Velocity_5_6DF5BD4448FA958C5E1D03A4550DEBD7` (break `/Game/Blueprints/BPS_MusicNote` _array_element_5)) true))
      (`AudioParameterControllerInterface.SetFloatArrayParameter` (`self.Audio`) "MelodyNotes" (`self.MelodyNotes`))
      (`AudioParameterControllerInterface.SetFloatArrayParameter` (`self.Audio`) "MelodyVelocities" (`self.MelodyVelocities`)))
    (:`then_8`
      (`AudioComponent.Play` _audio 0.0)
      (`AudioParameterControllerInterface.SetTriggerParameter` _audio "PlayMusic")
      (`KismetSystemLibrary.PrintString` "Should Play"))))

(fn `PopulateChordArrays`
  (params (Array :type "Array of /Game/Blueprints/BPS_ChordArrayWrapper Structure"))
  (for (_array_element _array_index) Array
    (for _index (range 6)
      (if (== _index 0)
        (if (`KismetArrayLibrary.Array_IsValidIndex` (break `/Game/Blueprints/BPS_ChordArrayWrapper` _array_element))
          (bind (_output_midinote _output_velocity) (break `/Game/Blueprints/BPS_MusicNote` (`|GetArrayItem` (break `/Game/Blueprints/BPS_ChordArrayWrapper` _array_element))))
          (`KismetArrayLibrary.Array_Set` (`self.ChordRoots`) _array_index _output_midinote true)
          (`KismetArrayLibrary.Array_Set` (`self.ChordRootVelocities`) _array_index _output_velocity true)
          (else
            (`KismetArrayLibrary.Array_Set` (`self.ChordRoots`) _array_index 0.0 true)
            (`KismetArrayLibrary.Array_Set` (`self.ChordRootVelocities`) _array_index 0.0 true)))
        (elif (== _index 1)
          (if (`KismetArrayLibrary.Array_IsValidIndex` (break `/Game/Blueprints/BPS_ChordArrayWrapper` _array_element) 1)
            (bind (_output_midinote_2 _output_velocity_2) (break `/Game/Blueprints/BPS_MusicNote` (`|GetArrayItem` (break `/Game/Blueprints/BPS_ChordArrayWrapper` _array_element) 1)))
            (`KismetArrayLibrary.Array_Set` (`self.Chord3rds`) _array_index _output_midinote_2 true)
            (`KismetArrayLibrary.Array_Set` (`self.Chord3rdVelocities`) _array_index _output_velocity_2 true)
            (else
              (`KismetArrayLibrary.Array_Set` (`self.Chord3rds`) _array_index 0.0 true)
              (`KismetArrayLibrary.Array_Set` (`self.Chord3rdVelocities`) _array_index 0.0 true)))
          (elif (== _index 2)
            (if (`KismetArrayLibrary.Array_IsValidIndex` (break `/Game/Blueprints/BPS_ChordArrayWrapper` _array_element) 2)
              (bind (_output_midinote_3 _output_velocity_3) (break `/Game/Blueprints/BPS_MusicNote` (`|GetArrayItem` (break `/Game/Blueprints/BPS_ChordArrayWrapper` _array_element) 2)))
              (`KismetArrayLibrary.Array_Set` (`self.Chord5ths`) _array_index _output_midinote_3 true)
              (`KismetArrayLibrary.Array_Set` (`self.Chord5thVelocities`) _array_index _output_velocity_3 true)
              (else
                (`KismetArrayLibrary.Array_Set` (`self.Chord5ths`) _array_index 0.0 true)
                (`KismetArrayLibrary.Array_Set` (`self.Chord5thVelocities`) _array_index 0.0 true)))
            (elif (== _index 3)
              (if (`KismetArrayLibrary.Array_IsValidIndex` (break `/Game/Blueprints/BPS_ChordArrayWrapper` _array_element) 3)
                (bind (_output_midinote_4 _output_velocity_4) (break `/Game/Blueprints/BPS_MusicNote` (`|GetArrayItem` (break `/Game/Blueprints/BPS_ChordArrayWrapper` _array_element) 3)))
                (`KismetArrayLibrary.Array_Set` (`self.Chord7ths`) _array_index _output_midinote_4 true)
                (`KismetArrayLibrary.Array_Set` (`self.Chord7thVelocities`) _array_index _output_velocity_4 true)
                (else
                  (`KismetArrayLibrary.Array_Set` (`self.Chord7ths`) _array_index 0.0 true)
                  (`KismetArrayLibrary.Array_Set` (`self.Chord7thVelocities`) _array_index 0.0 true)))
              (elif (== _index 4)
                (if (`KismetArrayLibrary.Array_IsValidIndex` (break `/Game/Blueprints/BPS_ChordArrayWrapper` _array_element) 4)
                  (bind (_output_midinote_5 _output_velocity_5) (break `/Game/Blueprints/BPS_MusicNote` (`|GetArrayItem` (break `/Game/Blueprints/BPS_ChordArrayWrapper` _array_element) 4)))
                  (`KismetArrayLibrary.Array_Set` (`self.Chord9ths`) _array_index _output_midinote_5 true)
                  (`KismetArrayLibrary.Array_Set` (`self.Chord9thVelocities`) _array_index _output_velocity_5 true)
                  (else
                    (`KismetArrayLibrary.Array_Set` (`self.Chord9ths`) _array_index 0.0 true)
                    (`KismetArrayLibrary.Array_Set` (`self.Chord9thVelocities`) _array_index 0.0 true)))
                (elif (== _index 5)
                  (if (`KismetArrayLibrary.Array_IsValidIndex` (break `/Game/Blueprints/BPS_ChordArrayWrapper` _array_element) 5)
                    (bind (_output_midinote_6 _output_velocity_6) (break `/Game/Blueprints/BPS_MusicNote` (`|GetArrayItem` (break `/Game/Blueprints/BPS_ChordArrayWrapper` _array_element) 5)))
                    (`KismetArrayLibrary.Array_Set` (`self.Chord9ths`) _array_index _output_midinote_6 true)
                    (`KismetArrayLibrary.Array_Set` (`self.Chord9thVelocities`) _array_index _output_velocity_6 true)
                    (else
                      (`KismetArrayLibrary.Array_Set` (`self.Chord9ths`) _array_index 0.0 true)
                      (`KismetArrayLibrary.Array_Set` (`self.Chord9thVelocities`) _array_index 0.0 true))))))))))))

(fn `UserConstructionScript`
  (bind _returnvalue (`|GenericCreateObject` "/Game/Blueprints/BP_DrumAndBassGenerator.BP_DrumAndBassGenerator_C"))
  (set `self.DrumAndBassGenerator` _returnvalue))