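; Game mode for an interactive drum-and-bass machine that opens a mouse-driven UI and plays an audio component.
; A 190 BPM Quartz clock starts playback on a bar boundary and raises a bar event.
; Accepted actions wait in a queue until the bar counter reaches its threshold.
; The queue then flushes, firing trigger parameters that randomize hi-hat roll, percussion, bass or lead channels in musical time.
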(event `self.ReceiveBeginPlay`
  (bind _returnvalue (`GameplayStatics.GetPlayerController` 0))
  (`self.Create and Start Quartz Clock`)
  (bind _returnvalue_2 (`|CreateWidget` (`self.UI`) _returnvalue))
  (`UserWidget.AddToViewport` _returnvalue_2 0)
  (`WidgetBlueprintLibrary.SetInputMode_UIOnlyEx` _returnvalue null)
  (set `PlayerController.bShowMouseCursor` true _returnvalue)
  (bind _dnb (`self.DnB`)
    (:`then`
      (`ActorComponent.Activate` _dnb false)
      (`AudioComponent.PlayQuantized` :`self` _dnb :`InClockHandle` (`self.ClockHandle`) :`InQuantizationBoundary` (make `QuartzQuantizationBoundary` "Bar")))
    (:`else`)))

(event `CustomEvent`
  (params (ClockName :type Name) (QuantizationType :type "EQuartzCommandQuantization Enum" :default "Bar") (NumBars :type Integer) (Beat :type Integer) (BeatFraction :type "Float (single-precision)"))
  (bind _queue (`self.Queue`))
  (bind _output_get (set `self.NumBars` (+ (`self.NumBars`) 1)))
  (if (>= _output_get 4)
    (set `self.NumBars` 1)
    (for _array_element _queue
      (`self.ExecuteAction` _array_element))
    (`KismetArrayLibrary.Array_Clear` _queue)))

(fn `Accept Action`
  (params (Action :type "/Game/Blueprints/BPE_QueueChoices Enum" :default "NewEnumerator9"))
  (`KismetArrayLibrary.Array_Add` (`self.Queue`) Action))

(fn `Create and Start Quartz Clock`
  (bind _returnvalue (`QuartzSubsystem.CreateNewClock` :`self` (subsystem `QuartzSubsystem`) :`ClockName` "DnB"))
  (bind _output_get (set `self.ClockHandle` _returnvalue))
  (bind _clockhandle (`QuartzClockHandle.SetBeatsPerMinute` :`self` _output_get :`BeatsPerMinute` 190.0))
  (bind _clockhandle_2 (`QuartzClockHandle.SubscribeToQuantizationEvent` _clockhandle "Bar" (`|CreateDelegate` :!event `CustomEvent`)))
  (`QuartzClockHandle.StartClock` _clockhandle_2))

(fn `ExecuteAction`
  (params (Action :type "/Game/Blueprints/BPE_QueueChoices Enum" :default "NewEnumerator0"))
  (switch `/Game/Blueprints/BPE_QueueChoices` Action
    (:`NewEnumerator9`
      (`self.RandomizeChannel` "RandomizeHHRoll"))
    (:`NewEnumerator10`
      (`self.RandomizeChannel` "RandomizePerc1"))
    (:`NewEnumerator11`
      (`self.RandomizeChannel` "RandomizePerc2"))
    (:`NewEnumerator12`
      (`self.RandomizeChannel` "RandomizeBassPad"))
    (:`NewEnumerator13`
      (`self.RandomizeChannel` "RandomizeLead"))))

(fn `RandomizeChannel`
  (params (TriggerName :type Name))
  (bind _dnb (`self.DnB`)
    (:`then`
      (`AudioParameterControllerInterface.SetTriggerParameter` _dnb TriggerName))
    (:`else`)))

(fn `UserConstructionScript`)